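; Homing projectile, apparently fired by a roaming slime enemy, that chases the VR player.
; On BeginPlay it sets the ProjectileMovement homing target to the HitBox of the player's VRPawn.
; Its Hitbox overlap applies fixed damage to actors tagged Player and destroys the bullet on anything else, so a player hit does not destroy it.
; An unconnected snippet would instead home on a component of the 1911 pistol.
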(event `self.ReceiveBeginPlay`
  ;[1 1 1] homing
  (bind _asvrpawn (cast `/Game/VRTemplate/Blueprints/VRPawn` (`GameplayStatics.GetPlayerPawn` 0)))
  (set `ProjectileMovementComponent.HomingTargetComponent` (`/Game/VRTemplate/Blueprints/VRPawn.HitBox` _asvrpawn) (`self.ProjectileMovement`)))

(event `self.Hitbox.OnComponentBeginOverlap`
  (params (OverlappedComponent :type "PrimitiveComponent Object Reference") (OtherActor :type "Actor Object Reference") (OtherComp :type "PrimitiveComponent Object Reference") (OtherBodyIndex :type Integer) (bFromSweep :type Boolean) (SweepResult :type "HitResult Structure (by ref)"))
  (if (`self.ActorHasTag` OtherActor "Player")
    (`GameplayStatics.ApplyDamage` OtherActor 35.0)
    (else
      (`self.K2_DestroyActor`))))

(fn `UserConstructionScript`)