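; BP_SlidingDoor is an interactable door that slides vertically in response to a crank wheel.
; On BeginPlay it records the Cube's starting height, casts its Activator to BP_CrankWheel and binds to that wheel's CrankRotating dispatcher.
; Each broadcast adds the Rotation value to the Cube's world Z, clamped between the start height and a fixed limit above it.
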(event `self.ReceiveBeginPlay`
  (bind (_returnvalue_x _returnvalue_y _returnvalue_z) (`KismetMathLibrary.BreakVector` (`SceneComponent.K2_GetComponentLocation` (`self.Cube`))))
  (set `self.StartZ` _returnvalue_z)
  (bind _asbp_crank_wheel (cast `/Game/CustomContent/Interactables/BP_CrankWheel` (`self.Activator`)))
  (add `/Game/CustomContent/Interactables/BP_CrankWheel.CrankRotating` _asbp_crank_wheel (delegate `CrankRotating_Event`)))

(event `CrankRotating_Event`
  (params (Rotation :type "Float (double-precision)"))
  (bind _cube (`self.Cube`))
  (bind _startz (`self.StartZ`))
  (bind (_returnvalue_x _returnvalue_y _returnvalue_z) (`KismetMathLibrary.BreakVector` (`SceneComponent.K2_GetComponentLocation` _cube)))
  (`SceneComponent.K2_SetWorldLocation` _cube (`KismetMathLibrary.MakeVector` _returnvalue_x _returnvalue_y (`KismetMathLibrary.FClamp` (+ Rotation _returnvalue_z) _startz (+ _startz 200.0))) false false))

(fn `UserConstructionScript`)