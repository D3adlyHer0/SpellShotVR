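; BP_LootTest is a test loot drop actor that displays an item's rarity and loot score.
; The construction script picks the sphere's material from ItemDetails.Rarity and writes ItemDetails.LootScore to a text render.
; On BeginPlay, the sphere gets a strong upward impulse with random horizontal spread to pop the loot out; the short delay that follows triggers nothing.
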(event `self.ReceiveBeginPlay`
  (bind _returnvalue (`KismetMathLibrary.RandomFloatInRange` -500.0 500.0))
  (`PrimitiveComponent.AddImpulse` (`self.Sphere`) (`KismetMathLibrary.MakeVector` _returnvalue _returnvalue 1500.0) "None" false)
  (`KismetSystemLibrary.Delay` 0.2))

(fn `UserConstructionScript`
  (bind (_rarity _lootscore) (break `/Game/CustomContent/LootGenerationStuff/Item_Struct` (`self.ItemDetails`)))
  (`PrimitiveComponent.SetMaterial` (`self.Sphere`) 0 (select `/Game/CustomContent/LootGenerationStuff/Rarity_Enum` _rarity :`NewEnumerator0` "/Game/FPWeapon/Materials/BaseMaterial.BaseMaterial" :`NewEnumerator1` "/Game/StarterContent/Materials/M_Ground_Grass.M_Ground_Grass" :`NewEnumerator2` "/Game/StarterContent/Blueprints/Assets/M_LightStage_Skybox_HDRI.M_LightStage_Skybox_HDRI" :`NewEnumerator3` "/Game/StarterContent/Materials/M_Metal_Chrome.M_Metal_Chrome" :`NewEnumerator4` "/Game/StarterContent/Materials/M_Metal_Gold.M_Metal_Gold" :!type "MaterialInterface Object Reference"))
  (`TextRenderComponent.K2_SetText` (`self.TextRender`) (`KismetTextLibrary.Conv_IntToText` _lootscore)))