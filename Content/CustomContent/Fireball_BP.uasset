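; A grabbable fireball spell projectile that arms shortly after being dropped and explodes on overlapping a non-projectile actor.
; The ActiveSpell actor's Increase event grows the explosion scale, while its Clock event is bound but empty.
; On impact, the collision sphere expands to that scale, FX spawn, spell level resets, and overlapping actors take damage after a brief delay.
; Tick orients the sphere along its velocity.
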(event `self.ReceiveBeginPlay`
  (bind _returnvalue (`GameplayStatics.GetActorOfClass` "/Game/CustomContent/SpellCastingStuff/ActiveSpell.ActiveSpell_C"))
  (bind _output_get (set `self.ActiveSpelll` _returnvalue))
  (add `/Game/CustomContent/SpellCastingStuff/ActiveSpell.Increase` _output_get (delegate `Increase`))
  (add `/Game/CustomContent/SpellCastingStuff/ActiveSpell.Clock` _output_get (delegate `Clock`)))

(event `Clock`
  ;[1 1 1] MakeLingeringDamage
)

(event `Increase`
  (set `self.ExplosionScale` (+ (`self.ExplosionScale`) (0.5 0.5 0.5))))

(event `self.ReceiveTick`
  (params (DeltaSeconds :type "Float (single-precision)"))
  (bind _sphere (`self.Sphere`))
  (bind _returnvalue (`SceneComponent.K2_GetComponentLocation` _sphere))
  (bind (_returnvalue_roll _returnvalue_pitch _returnvalue_yaw) (`KismetMathLibrary.BreakRotator` (`KismetMathLibrary.FindLookAtRotation` (+ (`SceneComponent.GetComponentVelocity` _sphere) _returnvalue) _returnvalue)))
  ;[1 1 1] Rotate
  (`SceneComponent.K2_SetWorldRotation` _sphere (`KismetMathLibrary.MakeRotator` _returnvalue_roll (+ _returnvalue_pitch -90.0) _returnvalue_yaw) false false))

(event `self.CrashSphere.OnComponentBeginOverlap`
  (params (OverlappedComponent :type "PrimitiveComponent Object Reference") (OtherActor :type "Actor Object Reference") (OtherComp :type "PrimitiveComponent Object Reference") (OtherBodyIndex :type Integer) (bFromSweep :type Boolean) (SweepResult :type "HitResult Structure (by ref)"))
  (if (`self.Primed`)
    (if (not (`self.ActorHasTag` OtherActor "Projectile"))
      (`PrimitiveComponent.SetSimulatePhysics` (`self.Sphere`) false)
      ;[1 0 0.2174] Change depending On Spells drawn
      (`SceneComponent.SetWorldScale3D` (`self.CrashSphere`) (`self.ExplosionScale`))
      (`self.Explode`))))

(event `Explode`
  (`NiagaraFunctionLibrary.SpawnSystemAtLocation` "/Game/CustomContent/Explosion_FX.Explosion_FX" (.location (`SceneComponent.K2_GetComponentToWorld` (`self.CrashSphere`))) (struct) (+ (`self.Effects Scale`) (/ (`self.ExplosionScale`) (5.0 55.0 5.0))))
  (set `/Game/CustomContent/SpellCastingStuff/ActiveSpell.SpellLevel` 0 (`self.ActiveSpelll`))
  (`KismetSystemLibrary.Delay` 0.2)
  (for _array_element (`PrimitiveComponent.GetOverlappingActors` (`self.CrashSphere`) null)
    (`GameplayStatics.ApplyDamage` _array_element (`self.Explosion Damage`) null (`GameplayStatics.GetPlayerPawn` 0)))
  (`ActorComponent.K2_DestroyComponent` (`self.CrashSphere`)))

(event `self.GrabComponent.OnGrabbed`
  (params (MotionController :type "MotionControllerComponent Object Reference") (MotionControllerAim :type "MotionControllerComponent Object Reference")))

(event `self.GrabComponent.OnDropped`
  (`PrimitiveComponent.SetSimulatePhysics` (`self.Sphere`) true)
  (`KismetSystemLibrary.Delay` 0.1)
  (set `self.Primed` true))

(fn `UserConstructionScript`)