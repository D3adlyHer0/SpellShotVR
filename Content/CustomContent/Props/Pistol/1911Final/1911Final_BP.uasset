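; 1911 pistol prop Blueprint that displays its loot score and rarity as an item.
; The construction script writes the LootScore from ItemDetails to a text render component.
; It also sets the Color variable of the RarityBeamFX effect by selecting a color for the item's rarity tier.
; The event graph is inactive, and a rarity-based material select is left unconnected.
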(fn `UserConstructionScript`
  (bind (_rarity _lootscore) (break `/Game/CustomContent/LootGenerationStuff/Item_Struct` (`self.Item Details`)))
  (`TextRenderComponent.K2_SetText` (`self.TextRender`) (`KismetTextLibrary.Conv_IntToText` _lootscore))
  (`NiagaraComponent.SetVariableLinearColor` (`self.RarityBeam_FX`) "Color" (select `/Game/CustomContent/LootGenerationStuff/Rarity_Enum` _rarity :`NewEnumerator0` (`self.CommonColor`) :`NewEnumerator1` (`self.UncommonColor`) :`NewEnumerator2` (`self.RareColor`) :`NewEnumerator3` (`self.Very RareColor`) :`NewEnumerator4` (`self.LegendaryColor`))))