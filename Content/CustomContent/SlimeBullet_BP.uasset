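; SlimeBullet_BP is a homing projectile that damages actors tagged Player.
; On BeginPlay it sets its ProjectileMovement homing target to the first child component of 1911Bottom on the 1911Final_BP pistol actor.
; Hitbox overlaps apply fixed damage to Player-tagged actors without destroying the bullet; any other overlap destroys it.
; An unconnected branch would instead home on the VRPawn's HitBox.
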(event `self.ReceiveBeginPlay`
  (bind _returnvalue (`GameplayStatics.GetActorOfClass` "/Game/CustomContent/Props/Pistol/1911Final/1911Final_BP.1911Final_BP_C"))
  (set `ProjectileMovementComponent.HomingTargetComponent` (`SceneComponent.GetChildComponent` (`/Game/CustomContent/Props/Pistol/1911Final/1911Final_BP.1911Bottom` _returnvalue) 0) (`self.ProjectileMovement`)))

(event `self.Hitbox.OnComponentBeginOverlap`
  (params (OverlappedComponent :type "PrimitiveComponent Object Reference") (OtherActor :type "Actor Object Reference") (OtherComp :type "PrimitiveComponent Object Reference") (OtherBodyIndex :type Integer) (bFromSweep :type Boolean) (SweepResult :type "HitResult Structure (by ref)"))
  (if (`self.ActorHasTag` OtherActor "Player")
    (`GameplayStatics.ApplyDamage` OtherActor 20.0)
    (else
      (`self.K2_DestroyActor`))))

(fn `UserConstructionScript`)