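; Chain lightning spell actor that visually arcs a Niagara beam between actors tagged "Enemy", with debug prints and no damage logic.
; BeginPlay fills NotHitYet, then calls CastSpell after a delay.
; CastSpell re-calls itself on a short delay, aiming LightingFX from the sphere, then LastHitLocation, at the nearest remaining enemy, which it removes.
; Chains only decrements on the first arc; later LastHitLocation updates re-query after removal, skipping ahead one target.
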(event `self.ReceiveBeginPlay`
  (bind _outactors (`GameplayStatics.GetAllActorsWithTag` "Enemy"))
  (for _array_element _outactors
    (`KismetArrayLibrary.Array_Add` (`self.NotHitYet`) _array_element)
    (`KismetSystemLibrary.PrintString` (`KismetSystemLibrary.GetDisplayName` _array_element)))
  (`KismetSystemLibrary.Delay` 1.0)
  (`KismetSystemLibrary.PrintString` "cast spell" true true (struct :`A` 1.0) 10.0)
  (`self.CastSpell`))

(event `CastSpell`
  (bind _nothityet (`self.NotHitYet`))
  (bind _nothityet_2 (`self.NotHitYet`))
  (bind (_distance _returnvalue) (`GameplayStatics.FindNearestActor` (`self.LastHitLocation`) (`self.NotHitYet`)))
  (bind _returnvalue_2 (`SceneComponent.K2_GetComponentLocation` (`self.Sphere`)))
  (bind (_distance_2 _returnvalue_3) (`GameplayStatics.FindNearestActor` _returnvalue_2 (`self.NotHitYet`)))
  (bind _returnvalue_location (`KismetMathLibrary.BreakTransform` (`self.GetTransform` _returnvalue)))
  (bind _returnvalue_location_2 (`KismetMathLibrary.BreakTransform` (`self.GetTransform` _returnvalue_3)))
  (if (`self.FirstBranch`)
    (`NiagaraComponent.SetNiagaraVariableVec3` (`self.Lighting_FX`) "StartPoint" _returnvalue_2)
    (`KismetSystemLibrary.PrintString` (`KismetSystemLibrary.GetDisplayName` _returnvalue_3))
    (set `self.LastHitLocation` _returnvalue_location_2)
    (`NiagaraComponent.SetNiagaraVariableVec3` (`self.Lighting_FX`) "EndPoint" (- _returnvalue_location_2 _returnvalue_2))
    (`KismetArrayLibrary.Array_Remove` _nothityet_2 (`KismetArrayLibrary.Array_Find` _nothityet_2 _returnvalue_3))
    (set `self.FirstBranch` false)
    (set `self.Chains` (- (`self.Chains`) 1.0))
    (`KismetSystemLibrary.Delay` 0.3)
    (`self.CastSpell`)
    (elif (>= (`self.Chains`) 1.0)
      (if (> (`KismetArrayLibrary.Array_Length` (`self.NotHitYet`)) 0)
        (`NiagaraComponent.SetNiagaraVariableVec3` (`self.Lighting_FX`) "StartPoint" (`self.LastHitLocation`))
        (`KismetSystemLibrary.PrintString` (`KismetStringLibrary.Conv_VectorToString` _returnvalue_location) true true (struct :`G` 0.66 :`B` 1.0 :`A` 1.0) 10.0)
        (`NiagaraComponent.SetNiagaraVariableVec3` (`self.Lighting_FX`) "EndPoint" _returnvalue_location)
        (`KismetArrayLibrary.Array_Remove` _nothityet (`KismetArrayLibrary.Array_Find` _nothityet _returnvalue))
        (set `self.LastHitLocation` _returnvalue_location)
        (`KismetSystemLibrary.Delay` 0.3)
        (`self.CastSpell`)))))

(fn `UserConstructionScript`)