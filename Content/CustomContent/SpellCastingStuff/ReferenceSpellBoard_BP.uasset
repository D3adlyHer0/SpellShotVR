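; Reference spell board actor that samples a drawn spline shape and exports it as a CSV point list with a Row Name header.
; On BeginPlay it takes 80 evenly spaced local-space points along the spline, draws a debug box at each, and stores them as text rows with X shifted by a fixed offset.
; After a short delay it overwrites savedLocations.csv at a hardcoded C: drive path and prints the result.
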(event `self.ReceiveBeginPlay`
  (set `self.SplineLength` (`SplineComponent.GetSplineLength` (`self.Spline`)))
  (`self.savelocation`)
  (`KismetSystemLibrary.Delay` 5.0)
  (`self.savetofile`))

(event `savelocation`
  (`KismetArrayLibrary.Array_Add` (`self.SvaedLocations`) (`KismetStringLibrary.Concat_StrStr` "Row Name" "," "X" "," "Y" "," "Z"))
  (for _index (range 1 81)
    (bind (_returnvalue_x _returnvalue_y _returnvalue_z) (`KismetMathLibrary.BreakVector` (`SplineComponent.GetLocationAtDistanceAlongSpline` (`self.Spline`) (* _index (/ (`self.SplineLength`) 80.0)) "Local")))
    (`KismetSystemLibrary.DrawDebugBox` (+ (`SceneComponent.K2_GetComponentLocation` (`self.DefaultSceneRoot`)) (`KismetMathLibrary.MakeVector` _returnvalue_x _returnvalue_y _returnvalue_z)) (2.0 2.0 2.0) (struct) (struct) 100.0)
    (`KismetArrayLibrary.Array_Add` (`self.SvaedLocations`) (`KismetStringLibrary.Concat_StrStr` (`KismetStringLibrary.Conv_IntToString` _index) "," (`KismetStringLibrary.Conv_DoubleToString` (+ _returnvalue_x 50.0)) "," (`KismetStringLibrary.Conv_DoubleToString` _returnvalue_y) "," (`KismetStringLibrary.Conv_DoubleToString` _returnvalue_z)))))

(event `savetofile`
  (bind _returnvalue (`self.FileIO__SaveStringArrayToFile` "C:\\test" "savedLocations.csv" (`self.SvaedLocations`) true))
  (if _returnvalue
    (`KismetSystemLibrary.PrintString` "Wrote to file")
    (else
      (`KismetSystemLibrary.PrintString` "Failed to write"))))

(fn `UserConstructionScript`)